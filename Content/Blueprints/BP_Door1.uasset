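; BP_Door1 is an interactable door that swings open once and supplies a prompt through GetInteractText.
; On first interaction it plays a swing sound, stores its yaw and uses DoorOpenTimeline to lerp from its current rotation toward that yaw plus 90 degrees.
; Once IsOpen is set, further interactions only play the locked sound twice, briefly spaced.
; A player HasKey check exists but is unconnected, so no key is required.
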(event `self.Interactor`
  (params (Actor :type "Actor Object Reference"))
  (bind _returnvalue (`self.K2_GetActorRotation`))
  (if (`self.IsOpen`)
    (`GameplayStatics.PlaySound2D` "/Game/Audio/S_DoorLocked.S_DoorLocked" 1.0 1.0 0.0 null null)
    (`KismetSystemLibrary.Delay` 0.25)
    (`GameplayStatics.PlaySound2D` "/Game/Audio/S_DoorLocked.S_DoorLocked" 1.0 1.0 0.0 null null)
    (else
      (`GameplayStatics.PlaySound2D` "/Game/Audio/S_DoorSwing.S_DoorSwing" 1.0 1.0 0.0 null null)
      (set `self.OpenAmount` (.yaw (`self.K2_GetActorRotation`)))
      (set `self.IsOpen` true)
      (bind (_direction _alpha) (`Timeline|DoorOpenTimeline`)
        (:`Update`
          (`self.K2_SetActorRotation` (`KismetMathLibrary.RLerp` _returnvalue (`KismetMathLibrary.MakeRotator` (.roll _returnvalue) (.pitch _returnvalue) (+ (`self.OpenAmount`) 90.0)) _alpha true)))))))

(fn `GetInteractText`
  (returns (InteractText :type Text))
  (return (`self.InteractText_0`)))

(fn `UserConstructionScript`)