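; BP_Shutdown is an interactable button that shuts down the game.
; On interaction it plays a turn-off sound, fades the camera and audio out, waits briefly, then quits.
; Tick refreshes the prompt text returned by GetInteractText.
; Both disabled-state checks are hard-wired false, so the button always acts as enabled.
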(event `self.ReceiveTick`
  (params (DeltaSeconds :type "Float (single-precision)"))
  (if false
    (set `self.Text` "The button is disabled")
    (else
      (set `self.Text` "Press E to shut down"))))

(event `/Game/FirstPerson/Blueprints/BPI_Interactable.Interactor`
  (params (Actor :type "Actor Object Reference"))
  (if (not false)
    (`GameplayStatics.PlaySound2D` "/Game/Audio/S_TurnOff.S_TurnOff" 1.0 1.0 0.0 null null false)
    (`PlayerCameraManager.StartCameraFade` :`self` (`PlayerController.PlayerCameraManager` (`GameplayStatics.GetPlayerController` 0)) :`ToAlpha` 1.0 :`Duration` 2.0 :`bShouldFadeAudio` true :`bHoldWhenFinished` true)
    (`KismetSystemLibrary.Delay` 4.0)
    (`KismetSystemLibrary.QuitGame` null "Quit")))

(fn `GetInteractText`
  (returns (InteractText :type Text))
  (return (`self.Text`)))

(fn `UserConstructionScript`)